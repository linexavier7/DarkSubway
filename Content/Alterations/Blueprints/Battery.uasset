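; Battery pickup actor that recharges the player's flashlight when interacted with.
; The OpenClose event finds the first FirstPersonCharacter_3 in the level, tops its BatteryFlashLight up to full, plays a charge sound at the capsule and destroys the pickup.
; The capsule's overlap event only casts to the player character and has no further effect.
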(event `/Game/Alterations/Blueprints/OpenClose.OpenClose`
  ;[1 1 1] Pegar bateria com interação
  (bind _outactors (`GameplayStatics.GetAllActorsOfClass` "/Game/FirstPersonBP/Blueprints/FirstPersonCharacter_3.FirstPersonCharacter_3_C"))
  (bind _output (`|GetArrayItem` _outactors))
  (bind _batteryflashlight (`/Game/FirstPersonBP/Blueprints/FirstPersonCharacter_3.BatteryFlashLight` _output))
  (set `/Game/FirstPersonBP/Blueprints/FirstPersonCharacter_3.BatteryFlashLight` (+ _batteryflashlight (- 100.0 _batteryflashlight)) _output)
  (`GameplayStatics.PlaySoundAtLocation` "/Game/Sound/Battery_Charge.Battery_Charge" (`SceneComponent.K2_GetComponentLocation` (`self.Capsule`)) (struct) 1.0 1.0 0.0 null null null null)
  (`self.K2_DestroyActor`))

(event `self.Capsule.OnComponentBeginOverlap`
  (params (OverlappedComponent :type "PrimitiveComponent Object Reference") (OtherActor :type "Actor Object Reference") (OtherComp :type "PrimitiveComponent Object Reference") (OtherBodyIndex :type Integer) (bFromSweep :type Boolean) (SweepResult :type "HitResult Structure (by ref)"))
  ;[1 1 1] Contato com Player
  (cast `/Game/FirstPersonBP/Blueprints/FirstPersonCharacter_3` OtherActor))

(fn `UserConstructionScript`)