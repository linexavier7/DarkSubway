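; PickUpNote_BP2 is a readable paper note that the player can open and close when standing near it.
; A box overlap with FirstPersonCharacter_3 sets IsClose, which lets the OpenClose event toggle reading.
; Opening plays a paper sound and adds a PickUpNoteWidget_BP2 to the viewport; closing plays another sound and removes it.
; Leaving the box while reading closes the note automatically.
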(event `self.OpenClose`
  (if (`self.IsClose`)
    (`self.TPickUpNote`)))

(event `TPickUpNote`
  (if (`self.IsReading`)
    (`self.PullDownNote`)
    (else
      (`self.PickUpNote`))))

(event `PickUpNote`
  (`GameplayStatics.PlaySoundAtLocation` "/Game/Sound/Paper_Open.Paper_Open" (`SceneComponent.K2_GetComponentLocation` (`self.PaperNote`)) (struct) 1.0 1.0 0.0 null null null null)
  (bind _returnvalue (`|CreateWidget` "/Game/Alterations/Blueprints/PickUpNoteWidget_BP2.PickUpNoteWidget_BP2_C"))
  (`UserWidget.AddToViewport` _returnvalue 0)
  (set `self.IsReading` true))

(event `PullDownNote`
  (`GameplayStatics.PlaySoundAtLocation` "/Game/Sound/Paper_Close.Paper_Close" (`SceneComponent.K2_GetComponentLocation` (`self.PaperNote`)) (struct) 1.0 1.0 0.0 null null null null)
  (`Widget.RemoveFromParent` (stale `PickUpNote` _returnvalue))
  (set `self.IsReading` false))

(event `self.Box.OnComponentBeginOverlap`
  (params (OverlappedComponent :type "PrimitiveComponent Object Reference") (OtherActor :type "Actor Object Reference") (OtherComp :type "PrimitiveComponent Object Reference") (OtherBodyIndex :type Integer) (bFromSweep :type Boolean) (SweepResult :type "HitResult Structure (by ref)"))
  (cast `/Game/FirstPersonBP/Blueprints/FirstPersonCharacter_3` OtherActor)
  (set `self.IsClose` true))

(event `self.Box.OnComponentEndOverlap`
  (params (OverlappedComponent :type "PrimitiveComponent Object Reference") (OtherActor :type "Actor Object Reference") (OtherComp :type "PrimitiveComponent Object Reference") (OtherBodyIndex :type Integer))
  (cast `/Game/FirstPersonBP/Blueprints/FirstPersonCharacter_3` OtherActor)
  (`|ExecutionSequence`
    (:`then_0`
      (set `self.IsClose` false)
      (if (`self.IsReading`)
        (`self.PullDownNote`)))))

(fn `UserConstructionScript`)