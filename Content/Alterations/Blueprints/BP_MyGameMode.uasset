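; Game mode that handles player respawning, the objective HUD and level progression.
; RespawnPlayer spawns a FirstPersonCharacter_3 at a given transform and has the first player controller possess it.
; BeginPlay adds the objective widget to the viewport, but the node storing its reference is disconnected.
; AdvancedLevel increments a level counter and switches on it to open one of three named levels, with a counter reset in the last branch.
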(event `RespawnPlayer`
  (params (SpawnTransform :type "Transform Structure"))
  (bind _returnvalue (`|SpawnActorFromClass` "/Game/FirstPersonBP/Blueprints/FirstPersonCharacter_3.FirstPersonCharacter_3_C" SpawnTransform "Undefined" "MultiplyWithRoot" null null))
  (`Controller.Possess` (`GameplayStatics.GetPlayerController` 0) _returnvalue))

(event `self.ReceiveBeginPlay`
  (bind _returnvalue (`|CreateWidget` "/Game/Alterations/Blueprints/BP_ObjectiveWidget.BP_ObjectiveWidget_C" (`GameplayStatics.GetPlayerController` 0)))
  (`UserWidget.AddToViewport` _returnvalue 0))

(fn `AdvancedLevel`
  (bind _currentlevel (`self.CurrentLevel`))
  ;[1 0.7496 0.9374] Advance Level
  (bind _result (`/Engine/EditorBlueprintResources/StandardMacros.IncrementInt` _currentlevel)
    (:`  `
      (switch `int` _result
        (:`0`
          (`GameplayStatics.OpenLevel` "1Level")
          (`KismetSystemLibrary.PrintString` "Level1"))
        (:`1`
          (`GameplayStatics.OpenLevel` "2Level")
          (`KismetSystemLibrary.PrintString` "Level2"))
        (:`2`
          (`GameplayStatics.OpenLevel` "3Level")
          (if (>= _currentlevel 3)
            (set `self.CurrentLevel` 0)
            (`KismetSystemLibrary.PrintString` "LastLevel")))))))

(fn `UserConstructionScript`)