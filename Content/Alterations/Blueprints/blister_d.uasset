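; A blister actor that plays a beat sound and rewards flashlight battery to the player when destroyed.
; Each tick, and when the character hits its sphere, the Beat sound's pitch and volume are remapped from its distance to the player; the hit also clears the character's BeatExecute flag.
; On destruction it adds battery to the first FirstPersonCharacter_3 found, prints the level, spawns a destruct effect and plays a burn death sound.
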(event `self.Sphere.OnComponentHit`
  (params (HitComponent :type "PrimitiveComponent Object Reference") (OtherActor :type "Actor Object Reference") (OtherComp :type "PrimitiveComponent Object Reference") (NormalImpulse :type "Vector Structure") (Hit :type "HitResult Structure (by ref)"))
  (bind _returnvalue (`KismetMathLibrary.MapRangeClamped` (`KismetMathLibrary.Vector_Distance` (`self.K2_GetActorLocation`) (`self.K2_GetActorLocation` (`GameplayStatics.GetPlayerCharacter` 0))) 0.0 100.0 100.0 200.0))
  (bind _asfirst_person_character_3 (cast `/Game/FirstPersonBP/Blueprints/FirstPersonCharacter_3` OtherActor))
  (set `/Game/FirstPersonBP/Blueprints/FirstPersonCharacter_3.BeatExecute` false _asfirst_person_character_3)
  (`AudioComponent.SetPitchMultiplier` (`self.Beat`) _returnvalue :!label _label)
  (`AudioComponent.SetVolumeMultiplier` (`self.Beat`) _returnvalue))

(event `self.ReceiveTick`
  (params (DeltaSeconds :type "Float (single-precision)"))
  (goto _label))

(event `self.ReceiveDestroyed`
  (bind _returnvalue (`SceneComponent.K2_GetComponentLocation` (`self.blister`)))
  (bind _outactors (`GameplayStatics.GetAllActorsOfClass` "/Game/FirstPersonBP/Blueprints/FirstPersonCharacter_3.FirstPersonCharacter_3_C"))
  (bind _output (`|GetArrayItem` _outactors))
  (bind _batteryflashlight (`/Game/FirstPersonBP/Blueprints/FirstPersonCharacter_3.BatteryFlashLight` _output))
  (set `/Game/FirstPersonBP/Blueprints/FirstPersonCharacter_3.BatteryFlashLight` (+ _batteryflashlight 10.0) _output)
  (`KismetSystemLibrary.PrintString` (`KismetStringLibrary.Conv_DoubleToString` _batteryflashlight))
  (`|SpawnActorFromClass` "/Game/Alterations/Blueprints/Blister_destruct_VFX.Blister_destruct_VFX_C" (`KismetMathLibrary.Conv_VectorToTransform` _returnvalue) "Undefined" "MultiplyWithRoot" null null)
  (`GameplayStatics.PlaySoundAtLocation` "/Game/Alterations/Sound/blister_burn_dead.blister_burn_dead" _returnvalue (struct) 1.0 1.0 0.1 "/Game/Alterations/Sound/BacksSound.BacksSound" null null null))

(fn `UserConstructionScript`)